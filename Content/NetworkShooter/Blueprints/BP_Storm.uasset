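; Battle-royale style storm zone for a network shooter: a cylinder that moves and shrinks in phases and punishes players who leave it.
; A delay-driven loop lerps the actor toward a random XY point and scales the cylinder down, pausing between phases.
; The shrink factor grows each phase; shrinking stops at a final scale while movement continues.
; Living characters ending overlap with the cylinder are passed to the GameMode for respawn.
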(event OnComponentEndOverlap(Cylinder)
  (params (OverlappedComponent :type Primitive%20Component%20Object%20Reference) (OtherActor :type Actor%20Object%20Reference) (OtherComp :type Primitive%20Component%20Object%20Reference) (OtherBodyIndex :type Integer))
  (bind _asbp_third_person_character (Utilities|Casting|CastToBP_ThirdPersonCharacter OtherActor))
  (if (not (Variables|/Game/NetworkShooter/Blueprints/BP_ThirdPersonCharacter.BP_ThirdPersonCharacter_C|GetIsDead? _asbp_third_person_character))
    (CallFunction|KillPlayer _asbp_third_person_character)))

(event Custom|TransformStorm
  (bind _transformdelay (Variables|Default|GetTransformDelay))
  (CallFunction|FindNextLocation :!label _label)
  (Variables|Default|SetPreviousLocation (Transformation|GetActorLocation))
  (Variables|Default|SetPreviousScale (Variables|/Script/Engine.SceneComponent|GetRelativeScale3D (Variables|Default|GetCylinder)))
  (Variables|Default|SetLerpAlpha 0.0)
  (Transformation|SetActorLocation (Math|Vector|Lerp(Vector) (Variables|Default|GetPreviousLocation) (Variables|Default|GetNextLocation) (Variables|Default|GetLerpAlpha)) true false :!label _label_2)
  (if (Variables|Default|GetCanShrink?)
    (CallFunction|ShrinkbyLerp))
  (Utilities|FlowControl|Delay _transformdelay)
  (bind _output_get (Variables|Default|SetLerpAlpha (+ (/ _transformdelay (Variables|Default|GetTotalTimeOfMoving)) (Variables|Default|GetLerpAlpha))))
  (if (< _output_get 1.0)
    (goto _label_2)
    (else
      (Variables|Default|SetCanShrink? (> (.x (Variables|/Script/Engine.SceneComponent|GetRelativeScale3D (Variables|Default|GetCylinder))) (Variables|Default|GetFinalStormScale)))
      (Variables|Default|SetScaleShrinkFactor (* (Variables|Default|GetScaleShrinkFactor) 1.1))
      (Utilities|FlowControl|Delay (Variables|Default|GetDelayBetweenShrinking))
      (goto _label))))

(event Custom|Server%20FindGameMode
  (bind _asbp_third_person_game_mode (Utilities|Casting|CastToBP_ThirdPersonGameMode (Game|GetGameMode)))
  (Variables|Default|SetGameMode _asbp_third_person_game_mode))

(event Custom|KillPlayer
  (params (Player :type BP%20Third%20Person%20Character%20Object%20Reference))
  (Default|RespawnCharacter (Variables|Default|GetGameMode) Player))

(event EventBeginPlay
  (Variables|Default|SetCanShrink? true)
  (CallFunction|ServerFindGameMode)
  (CallFunction|TransformStorm))

(event EventTick
  (params (DeltaSeconds :type Float%20%28single-precision%29))
  (Development|PrintString (Utilities|String|Append "Loc:" (Utilities|String|ToString(Vector) (Transformation|GetActorLocation)) "Scale:" (Utilities|String|ToString(Vector) (Variables|/Script/Engine.SceneComponent|GetRelativeScale3D (Variables|Default|GetCylinder)))) true true "(R=0.000000,G=0.660000,B=1.000000,A=1.000000)" DeltaSeconds))

(fn ConstructionScript)

(fn FindNextLocation
  (Variables|Default|SetNextLocation (Math|Vector|MakeVector (Math|Random|RandomFloatinRange 0.0 (Variables|Default|GetRandomLocationRadius)) (Math|Random|RandomFloatinRange 0.0 (Variables|Default|GetRandomLocationRadius)) (.z (Transformation|GetActorLocation)))))

(fn ShrinkbyLerp
  (bind _previousscale (Variables|Default|GetPreviousScale))
  (bind _previousscale_2 (Variables|Default|GetPreviousScale))
  (bind _scaleshrinkfactor (Variables|Default|GetScaleShrinkFactor))
  (bind _lerpalpha (Variables|Default|GetLerpAlpha))
  (bind _returnvalue (/ _previousscale _scaleshrinkfactor))
  (bind _returnvalue_2 (Math|Vector|Lerp(Vector) _previousscale_2 _returnvalue _lerpalpha))
  (Transformation|SetRelativeScale3D (Variables|Default|GetCylinder) (Math|Vector|MakeVector (.x _returnvalue_2) (.y _returnvalue_2) (Variables|Default|GetDefaultStormHeight))))